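; Level trigger actor that plays a cutscene when the player character overlaps it.
; On overlap with PlayerCharacter_BP it disables player interaction, then creates and plays a Level Sequence player for the LevelSeqToUse sequence.
; A callback bound to the sequence's stop event re-enables player interaction when playback ends.
; Nothing in the graph guards against retriggering on later overlaps.
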(event Custom|CustomEvent
  ;[0.4963 1 0.4817] Spiller av cutscenen og lager en event når den er ferdig å spille av.
  (CallFunction|EnablePlayerInteraction))

(event EventBeginPlay)

(event Collision|EventActorBeginOverlap
  (params (OtherActor :type Actor%20Object%20Reference))
  (Utilities|Casting|CastToPlayerCharacter_BP OtherActor)
  (CallFunction|DisablePlayerInteraction)
  (bind _returnvalue (Sequencer|Player|CreateLevelSequencePlayer (Variables|Default|GetLevelSeqToUse)))
  ;[0.4963 1 0.4817] Spiller av cutscenen og lager en event når den er ferdig å spille av.
  (Sequencer|Player|Play _returnvalue :!class /Script/MovieScene.MovieSceneSequencePlayer)
  (EventDispatchers|AssignOnStop _returnvalue (delegate Custom|CustomEvent)))

(event EventTick
  (params (DeltaSeconds :type Float%20%28single-precision%29))
  (|CallParentFunction DeltaSeconds) ; This node is disabled and will not be called.\nDrag off pins to build functionality.
)

(fn ConstructionScript
  (|CallParentFunction))