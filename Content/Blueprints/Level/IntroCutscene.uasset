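; Level actor that plays a chosen intro Level Sequence on BeginPlay unless its indexed flag in GameModeBase's IntroCutsceneArray is already true.
; Before playback it inserts the negated flag at that index, intended to prevent replay when re-entering the room.
; It blocks movement, look and jump and hides cursor and HUD.
; When the sequence stops, it restores these, creating a fresh HUD widget, then destroys itself.
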(event Custom|OnStopPlay
  ;[0.4963 1 0.4817] Spiller av cutscenen og lager en event når den er ferdig å spille av, samt slettes actoren
  (CallFunction|EnablePlayerInteraction)
  (Development|PrintString (Utilities|String|ToString(Boolean) (Utilities|Array|Get(acopy) (Variables|/Game/Blueprints/GameModeBase.GameModeBase_C|GetIntroCutsceneArray (stale EventBeginPlay _asgame_mode_base_2)) (Variables|Default|GetPlayArray))))
  (Actor|DestroyActor))

(event EventBeginPlay
  (bind _playarray (Variables|Default|GetPlayArray))
  ;[0 1 0.02158] Når BeginPlay kjøres, spør vi om vi skal spille av cutscenen. Hvis den skal spilles av, returneres false fra GameMode og vi disabler player input
  (bind _asgame_mode_base (Utilities|Casting|CastToGameModeBase (Game|GetGameMode)))
  (Development|PrintString (Utilities|String|ToString(Boolean) (Utilities|Array|Get(acopy) (Variables|/Game/Blueprints/GameModeBase.GameModeBase_C|GetIntroCutsceneArray _asgame_mode_base) (Variables|Default|GetPlayArray))))
  (if (not (Utilities|Array|Get(acopy) (Variables|/Game/Blueprints/GameModeBase.GameModeBase_C|GetIntroCutsceneArray _asgame_mode_base) (Variables|Default|GetPlayArray)))
    (CallFunction|DisablePlayerInteraction)
    ;[1 1 1] Endrer på en boolean sånn at sequencen ikke spilles av neste gang du går inn i rommet
    (bind _asgame_mode_base_2 (Utilities|Casting|CastToGameModeBase (Game|GetGameMode)))
    (Utilities|Array|Insert (Variables|/Game/Blueprints/GameModeBase.GameModeBase_C|GetIntroCutsceneArray _asgame_mode_base_2) (not (Utilities|Array|Get(acopy) (Variables|/Game/Blueprints/GameModeBase.GameModeBase_C|GetIntroCutsceneArray _asgame_mode_base_2) _playarray)) _playarray)
    ;[0.4963 1 0.4817] Spiller av cutscenen og lager en event når den er ferdig å spille av, samt slettes actoren
    (bind _returnvalue (Sequencer|Player|CreateLevelSequencePlayer (Variables|Default|GetLevelSeqToUse)))
    (Sequencer|Player|Play _returnvalue :!class /Script/MovieScene.MovieSceneSequencePlayer)
    (EventDispatchers|AssignOnStop _returnvalue (delegate Custom|OnStopPlay))))

(event EventTick
  (params (DeltaSeconds :type Float%20%28single-precision%29)))

(event Collision|EventActorBeginOverlap
  (params (OtherActor :type Actor%20Object%20Reference)))

(fn ConstructionScript)

(fn DisablePlayerInteraction
  (Variables|Default|SetPlConRef (Game|GetPlayerController 0))
  (bind _asplayer_character_bp (Utilities|Casting|CastToPlayerCharacter_BP (Game|GetPlayerCharacter 0)))
  (bind _output_get (Variables|Default|SetPlayerRef _asplayer_character_bp))
  (Variables|/Script/Engine.Character|SetJumpMaxCount _output_get 0)
  (Variables|/Game/Blueprints/Character/PlayerCharacter_BP.PlayerCharacter_BP_C|SetisInCutscene (Variables|Default|GetPlayerRef) true)
  ;[0.9345 0.3694 1] Fjerner HUD fra viewport
  (bind _output_get_2 (Variables|Default|SetPlayerHUDRef (Variables|/Game/Blueprints/Character/PlayerCharacter_BP.PlayerCharacter_BP_C|GetHUD_reference (Variables|Default|GetPlayerRef))))
  (Widget|RemovefromParent _output_get_2)
  (Rendering|SetVisibility (Variables|/Script/Gruppe1.PlayerCharacter|GetCursorToWorld _output_get) false false)
  (Variables|/Script/Engine.PlayerController|SetbShowMouseCursor (Variables|Default|GetPlConRef) false)
  (Input|SetIgnoreMoveInput (Variables|Default|GetPlConRef) true)
  (Input|SetIgnoreLookInput (Variables|Default|GetPlConRef) true))

(fn EnablePlayerInteraction
  (bind _playerref (Variables|Default|GetPlayerRef))
  (Variables|/Script/Engine.Character|SetJumpMaxCount _playerref 1)
  (Variables|/Game/Blueprints/Character/PlayerCharacter_BP.PlayerCharacter_BP_C|SetisInCutscene _playerref false)
  (Input|SetIgnoreMoveInput (Variables|Default|GetPlConRef) false)
  (Input|SetIgnoreLookInput (Variables|Default|GetPlConRef) false)
  (Variables|/Script/Engine.PlayerController|SetbShowMouseCursor (Variables|Default|GetPlConRef) true)
  (Rendering|SetVisibility (Variables|/Script/Gruppe1.PlayerCharacter|GetCursorToWorld (Variables|Default|GetPlayerRef)) true false)
  ;[1 0.8642 0.1582] Gjør HUD visible igjen
  (bind _returnvalue (UserInterface|CreateWidget "/Game/UI/HUD.HUD_C" (Variables|Default|GetPlConRef)))
  (bind _output_get (Variables|Default|SetPlayerHUDRef _returnvalue))
  (UserInterface|Viewport|AddtoViewport _output_get 0))