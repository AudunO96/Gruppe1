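; Level intro actor that plays a configurable level sequence as an opening cutscene when play begins.
; On BeginPlay it removes the player's HUD, hides the cursor and cursor-to-world marker, disables jumping, ignores move and look input, and flags the player as in a cutscene.
; When the sequence stops, it restores those controls, zeroes the player's rotation and adds a newly created HUD widget to the viewport.
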(event Custom|OnStopPlay
  (bind _playerref (Variables|Default|GetPlayerRef))
  ;[0.4963 1 0.4817] Spiller av og kjører spesifikk behaviour når sequencen er ferdig.
  (Variables|/Script/Engine.Character|SetJumpMaxCount _playerref 1)
  (Variables|/Game/Blueprints/Character/PlayerCharacter_BP.PlayerCharacter_BP_C|SetisInCutscene _playerref false)
  (Input|SetIgnoreMoveInput (Variables|Default|GetPlConRef) false)
  (Input|SetIgnoreLookInput (Variables|Default|GetPlConRef) false)
  (Variables|/Script/Engine.PlayerController|SetbShowMouseCursor (Variables|Default|GetPlConRef) true)
  (Transformation|SetActorRotation (Variables|Default|GetPlayerRef))
  (Rendering|SetVisibility (Variables|/Script/Gruppe1.PlayerCharacter|GetCursorToWorld (stale EventBeginPlay _output_get)) true false)
  (bind _returnvalue (UserInterface|CreateWidget "/Game/UI/HUD.HUD_C" (Variables|Default|GetPlConRef)))
  (bind _output_get (Variables|Default|SetPlayerHUDRef _returnvalue))
  (UserInterface|Viewport|AddtoViewport _output_get 0))

(event EventBeginPlay
  (Variables|Default|SetPlConRef (Game|GetPlayerController 0))
  (bind _asplayer_character_bp (Utilities|Casting|CastToPlayerCharacter_BP (Game|GetPlayerCharacter 0)))
  (bind _output_get (Variables|Default|SetPlayerRef _asplayer_character_bp))
  (Variables|/Script/Engine.Character|SetJumpMaxCount _output_get 0)
  (Variables|/Game/Blueprints/Character/PlayerCharacter_BP.PlayerCharacter_BP_C|SetisInCutscene (Variables|Default|GetPlayerRef) true)
  (bind _output_get_2 (Variables|Default|SetPlayerHUDRef (Variables|/Game/Blueprints/Character/PlayerCharacter_BP.PlayerCharacter_BP_C|GetHUD_reference (Variables|Default|GetPlayerRef))))
  (Widget|RemovefromParent _output_get_2)
  (Rendering|SetVisibility (Variables|/Script/Gruppe1.PlayerCharacter|GetCursorToWorld _output_get) false false)
  (Variables|/Script/Engine.PlayerController|SetbShowMouseCursor (Variables|Default|GetPlConRef) false)
  (Input|SetIgnoreMoveInput (Variables|Default|GetPlConRef) true)
  (Input|SetIgnoreLookInput (Variables|Default|GetPlConRef) true)
  (bind _returnvalue (Sequencer|Player|CreateLevelSequencePlayer (Variables|Default|GetLevelSeqToUse)))
  ;[0.4963 1 0.4817] Spiller av og kjører spesifikk behaviour når sequencen er ferdig.
  (Sequencer|Player|Play _returnvalue :!class /Script/MovieScene.MovieSceneSequencePlayer)
  (EventDispatchers|AssignOnStop _returnvalue (delegate Custom|OnStopPlay)))

(event EventTick
  (params (DeltaSeconds :type Float%20%28single-precision%29)))

(event Collision|EventActorBeginOverlap
  (params (OtherActor :type Actor%20Object%20Reference)))

(fn ConstructionScript)