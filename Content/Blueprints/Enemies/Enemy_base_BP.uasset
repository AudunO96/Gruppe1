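; Base enemy Blueprint that manages a world health bar and responds to healing on overlap.
; On BeginPlay it hides the bar, initializes health and passes max and current health to the EnemyHealthBar widget.
; Overlapping a Healing_base actor reveals the bar, applies that actor's delivered healing and refreshes the display.
; Each tick turns the bar toward the player camera by copying its rotation with a 180-degree yaw offset.
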(event EventBeginPlay
  (bind _healthbar (Variables|Default|GetHealthBar))
  ;[1 1 1] Sets initial values
  (Rendering|SetVisibility _healthbar false false)
  (Class|EnemyBase|SetHealth)
  (bind _asenemy_health_bar (Utilities|Casting|CastToEnemyHealthBar (UserInterface|GetUserWidgetObject _healthbar)))
  (bind _output_get (Variables|Default|SetHealthbar%20reference _asenemy_health_bar))
  (bind _returnvalue (Class|EnemyBase|GetHealth))
  (bind _returnvalue_2 (Class|EnemyBase|GetMaxHealth))
  (Variables|/Game/Blueprints/HUD/EnemyHealthBar.EnemyHealthBar_C|SetmaxHealth _output_get _returnvalue_2)
  (Default|UpdateHealth _output_get _returnvalue))

(event Collision|EventActorBeginOverlap
  (params (OtherActor :type Actor%20Object%20Reference))
  ;[1 1 1] Deals with incoming damage
  ; TODO: Projectile overlap
  (bind _ashealing_base (Utilities|Casting|CastToHealing_base OtherActor))
  (bind _returnvalue (Class|HealingBase|DeliverHealing _ashealing_base 1.0))
  (Rendering|SetVisibility (Variables|Default|GetHealthBar) true false)
  (Class|EnemyBase|RecieveHealing _returnvalue)
  (bind _returnvalue_2 (Class|EnemyBase|GetHealth))
  (Default|UpdateHealth (Variables|Default|GetHealthbar%20reference) _returnvalue_2))

(event EventTick
  (params (DeltaSeconds :type Float%20%28single-precision%29))
  ;[1 1 1] Rotates healthbar to camera
  ; TODO: stop rolling
  (CallFunction|RotateHealthbartoCamera))

(fn ConstructionScript)

(fn RotateHealthbartoCamera
  (Transformation|SetWorldRotation (Variables|Default|GetHealthBar) (Math|Rotator|CombineRotators (Camera|GetCameraRotation (Game|GetPlayerCameraManager 0)) "180.000000, 0, 0") false false))