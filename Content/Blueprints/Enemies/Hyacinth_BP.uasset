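; Hyacinth is a summoner enemy that spawns foxes, or less often deer, at an offset from itself until its corruption is removed.
; BeginPlay reveals three crystals in sequence on staggered delays.
; Tick checks the enemy count and, at or below a minimum, flags casting and runs a randomly ending, max-capped loop that calls Summon through a Delay.
; OnRemoveCorruption marks it dead, blocking new casts.
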(event EventBeginPlay
  (|CallParentFunction)
  (Utilities|FlowControl|Delay 15.0)
  (Rendering|SetVisibility (Variables|/Script/Engine.Character|GetCapsuleComponent (Variables|Default|GetCrystal1)) true true)
  (Utilities|FlowControl|Delay 2e+01)
  (Rendering|SetVisibility (Variables|/Script/Engine.Character|GetCapsuleComponent (Variables|Default|GetCrystal2)) true true)
  (Utilities|FlowControl|Delay 25.0)
  (Rendering|SetVisibility (Variables|/Script/Engine.Character|GetCapsuleComponent (Variables|Default|GetCrystal3)) true true))

(event Collision|EventActorBeginOverlap
  (params (OtherActor :type Actor%20Object%20Reference))
  (|CallParentFunction OtherActor) ; This node is disabled and will not be called.\nDrag off pins to build functionality.
)

(event EventOnRemoveCorruption
  (Variables|Default|SetIsDead true))

(event EventTick
  (params (DeltaSeconds :type Float%20%28single-precision%29))
  (|CallParentFunction DeltaSeconds)
  (bind _outactors (Actor|GetAllActorsOfClass "/Script/Gruppe1.EnemyBase"))
  (if (and (<= (Utilities|Array|Length _outactors) (Variables|Default|GetMinEnemies)) (not (Variables|Default|GetIsDead)))
    (Variables|Default|SetIsCasting true)
    (while (and (<= (Utilities|Array|Length (stale _outactors_2)) (Variables|Default|GetMaxEnemies)) (<= (Math|Random|RandomInteger 100) 90))
      (bind _outactors_2 (Actor|GetAllActorsOfClass "/Game/Blueprints/Enemies/Enemy_base_BP.Enemy_base_BP_C"))
      (Utilities|FlowControl|Delay 1.0)
      (CallFunction|Summon))
    (Variables|Default|SetIsCasting false)))

(fn ConstructionScript
  (|CallParentFunction))

(fn Summon
  (bind _self self)
  (bind _spawnoffset (Variables|Default|GetSpawnOffset))
  (bind _returnvalue (Transformation|GetActorTransform _self))
  (bind (_location _rotation _scale) (Math|Transform|BreakTransform _returnvalue))
  (bind _returnvalue_2 (+ _location _spawnoffset))
  (bind _returnvalue_3 (Math|Transform|MakeTransform _returnvalue_2 _rotation _scale))
  (if (<= (Math|Random|RandomInteger 100) 15)
    (Game|SpawnActorfromClass "/Game/Blueprints/Enemies/Enemy_Deer_BP.Enemy_Deer_BP_C" _returnvalue_3 "Undefined" 0 _self)
    (else
      (Game|SpawnActorfromClass "/Game/Blueprints/Enemies/Enemy_Fox_BP.Enemy_Fox_BP_C" _returnvalue_3 "Undefined" 0 _self))))