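; Interactable dialogue actor that plays a multi-line conversation, one line per interaction.
; BeginPlay caches Dialogue_Text row names matching its DiaID.
; Interact advances LineCurrent, then shows the row matching ConvoID and line in a Dialogue_BP widget, removing it and resetting unless exactly one line is returned.
; Overlap shows a prompt text that rotates each tick to face the camera; the player leaving hides it and clears the dialogue.
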(event EventBeginPlay
  (bind _outrownames (DataTable|GetDataTableRowNames "/Game/Blueprints/Dialogue/Dialogue_Text.Dialogue_Text"))
  (for _array_element _outrownames
    (bind _returnvalue (Utilities|GetDataTableRow "/Game/Blueprints/Dialogue/Dialogue_Text.Dialogue_Text" _array_element)
      (:then
        (if (== (.Dia_ID (Utilities|Struct|BreakDialogueStruct _returnvalue)) (Variables|Default|GetDia_ID))
          (Utilities|Array|Add (Variables|Default|GetText) _array_element))))))

(event Collision|EventActorBeginOverlap
  (params (OtherActor :type Actor%20Object%20Reference))
  (Rendering|SetVisibility (Variables|Default|GetInfoText) true false))

(event EventTick
  (params (DeltaSeconds :type Float%20%28single-precision%29))
  (CallFunction|InfoTextRotation))

(event EventInteract
  (Math|Integer|IncrementInt (Variables|Default|GetLineCurrent)
    (:%20%20
      (CallFunction|DialogueCreate)
      (Rendering|SetVisibility (Variables|Default|GetInfoText) false false))))

(event Collision|EventActorEndOverlap
  (params (OtherActor :type Actor%20Object%20Reference))
  (Utilities|Casting|CastToPlayerCharacter OtherActor)
  (Widget|RemovefromParent (Variables|Default|GetDialogue%20Ref))
  (Variables|Default|SetDialogue%20Ref 0)
  (Variables|Default|SetLineCurrent 0)
  (Rendering|SetVisibility (Variables|Default|GetInfoText) false false))

(fn ConstructionScript)

(fn DialogueCreate
  (Utilities|IsValid (Variables|Default|GetDialogue%20Ref)
    (:Is%20Valid
      (bind _returnedline (CallFunction|DialogueGetLine))
      (Variables|/Game/Blueprints/Dialogue/Dialogue_BP.Dialogue_BP_C|SetDialogueText (Variables|Default|GetDialogue%20Ref) _returnedline))
    (:Is%20Not%20Valid
      (bind _returnvalue (UserInterface|CreateWidget "/Game/Blueprints/Dialogue/Dialogue_BP.Dialogue_BP_C" (Game|GetPlayerController 0)))
      (bind _output_get (Variables|Default|SetDialogue%20Ref _returnvalue))
      (UserInterface|Viewport|AddtoViewport _output_get 1)
      (bind _returnedline_2 (CallFunction|DialogueGetLine))
      (Variables|/Game/Blueprints/Dialogue/Dialogue_BP.Dialogue_BP_C|SetDialogueText (Variables|Default|GetDialogue%20Ref) _returnedline_2))))

(fn DialogueGetLine
  (for _array_element (Variables|Default|GetText)
    (bind _returnvalue (Utilities|GetDataTableRow "/Game/Blueprints/Dialogue/Dialogue_Text.Dialogue_Text" _array_element)
      (:then
        (if (and (== (.Convo_ID (Utilities|Struct|BreakDialogueStruct _returnvalue)) (Variables|Default|GetConvo_ID)) (== (.Line_ID (Utilities|Struct|BreakDialogueStruct _returnvalue)) (Variables|Default|GetLineCurrent)))
          (Utilities|Array|Add (LocalVariables|GetReturnedLines) (.Text (Utilities|Struct|BreakDialogueStruct _returnvalue)))))))
  (if (== (Utilities|Array|Length (LocalVariables|GetReturnedLines)) 1)
    (return (Utilities|Array|Get(acopy) (LocalVariables|GetReturnedLines)))
    (else
      ;[1 1 1] Setter tilbake til første linje og fjerner widgeten fra HUD
      (Widget|RemovefromParent (Variables|Default|GetDialogue%20Ref))
      (Variables|Default|SetDialogue%20Ref 0)
      (Variables|Default|SetLineCurrent 0))))

(fn InfoTextRotation
  (Transformation|SetWorldRotation (Variables|Default|GetInfoText) (Math|Rotator|CombineRotators (Camera|GetCameraRotation (Game|GetPlayerCameraManager 0)) "180.000000,0.000000,0.000000") false false))