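; OverlapDialogue_BP is an actor that shows a dialogue widget while the player character overlaps it.
; On begin overlap it creates a Dialogue_BP widget, stores it in DialogueReference, adds it to the viewport and sets its text from MyText.
; End overlap removes the widget and clears the reference.
; A begin overlap that finds an existing widget takes that same removal path instead of creating another.
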(event EventBeginPlay)

(event Collision|EventActorEndOverlap
  (params (OtherActor :type Actor%20Object%20Reference))
  (Utilities|Casting|CastToPlayerCharacter OtherActor)
  (Widget|RemovefromParent (Variables|Default|GetDialogueReference))
  (Variables|Default|SetDialogueReference 0))

(event Collision|EventActorBeginOverlap
  (params (OtherActor :type Actor%20Object%20Reference))
  (Utilities|Casting|CastToPlayerCharacter OtherActor)
  (Utilities|IsValid (Variables|Default|GetDialogueReference) ; Sjekker om den allerede eksisterer
    (:Is%20Valid
      (Widget|RemovefromParent (Variables|Default|GetDialogueReference))
      (Variables|Default|SetDialogueReference 0))
    (:Is%20Not%20Valid
      (bind _returnvalue (UserInterface|CreateWidget "/Game/Blueprints/Dialogue/Dialogue_BP.Dialogue_BP_C" (Game|GetPlayerController 0)))
      (bind _output_get (Variables|Default|SetDialogueReference _returnvalue))
      (UserInterface|Viewport|AddtoViewport _output_get 1)
      (Variables|/Game/Blueprints/Dialogue/Dialogue_BP.Dialogue_BP_C|SetDialogueText (Variables|Default|GetDialogueReference) (Variables|Default|GetMyText)))))

(event EventTick
  (params (DeltaSeconds :type Float%20%28single-precision%29)))

(fn ConstructionScript)