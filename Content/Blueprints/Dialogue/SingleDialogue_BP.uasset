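; SingleDialogue_BP is an interactable actor that shows a single piece of dialogue text to the player.
; Overlap shows a floating InfoText, which is rotated every tick to face the camera.
; Interact toggles a Dialogue_BP widget filled with MyText, creating it and hiding the prompt, or removing it if already open.
; When the PlayerCharacter leaves the overlap, the widget is removed and the prompt hidden.
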(event EventBeginPlay)

(event Collision|EventActorBeginOverlap
  (params (OtherActor :type Actor%20Object%20Reference))
  (Rendering|SetVisibility (Variables|Default|GetInfo%20Text) true false))

(event Collision|EventActorEndOverlap
  (params (OtherActor :type Actor%20Object%20Reference))
  (Utilities|Casting|CastToPlayerCharacter OtherActor)
  (Widget|RemovefromParent (Variables|Default|GetDialogueReference))
  (Variables|Default|SetDialogueReference 0)
  (Rendering|SetVisibility (Variables|Default|GetInfo%20Text) false false))

(event EventTick
  (params (DeltaSeconds :type Float%20%28single-precision%29))
  (CallFunction|SetRotationText))

(event EventInteract
  (Utilities|IsValid (Variables|Default|GetDialogueReference) ; Sjekker om den allerede eksisterer
    (:Is%20Valid
      (Widget|RemovefromParent (Variables|Default|GetDialogueReference))
      (Variables|Default|SetDialogueReference 0)
      (Rendering|SetVisibility (Variables|Default|GetInfo%20Text) false false))
    (:Is%20Not%20Valid
      (bind _returnvalue (UserInterface|CreateWidget "/Game/Blueprints/Dialogue/Dialogue_BP.Dialogue_BP_C" (Game|GetPlayerController 0)))
      (bind _output_get (Variables|Default|SetDialogueReference _returnvalue))
      (UserInterface|Viewport|AddtoViewport _output_get 1)
      (Variables|/Game/Blueprints/Dialogue/Dialogue_BP.Dialogue_BP_C|SetDialogueText (Variables|Default|GetDialogueReference) (Variables|Default|GetMyText))
      (Rendering|SetVisibility (Variables|Default|GetInfo%20Text) false false))))

(fn ConstructionScript)

(fn SetRotationText
  (Transformation|SetWorldRotation (Variables|Default|GetInfo%20Text) (Math|Rotator|CombineRotators (Camera|GetCameraRotation (Game|GetPlayerCameraManager 0)) "180.000000,0.000000,0.000000") false false))